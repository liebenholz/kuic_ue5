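; BP_moveLR is an actor Blueprint that slides its Sphere component back and forth along its relative X axis while playing.
; Tick advances XPosition at a constant, frame-rate-independent speed after a zero-length Delay, flipping IsLPosMovement at either end of a fixed range.
; The Play function sets the IsPlay flag that gates this movement and always returns false.
; An unconnected leftover movement snippet never runs.
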(event `self.ReceiveBeginPlay`)

(event `self.ReceiveTick`
  (params (DeltaSeconds :type "Float (single-precision)"))
  (if (`self.isPlay`)
    (if (`self.isLPosMovement`)
      ;[1 1 1] 왼쪽으로 한 번 움직이기
      (`KismetSystemLibrary.Delay` 0.0)
      (bind _output_get (set `self.xPosition` (+ (* DeltaSeconds 50.0) (`self.xPosition`))))
      (`SceneComponent.K2_SetRelativeLocation` (`self.Sphere`) (`KismetMathLibrary.MakeVector` _output_get) false false)
      (if (>= (`self.xPosition`) 200.0)
        (set `self.isLPosMovement` false))
      (else
        ;[1 1 1] 오른족으로 한 번 움직이기
        (`KismetSystemLibrary.Delay` 0.0)
        (bind _output_get_2 (set `self.xPosition` (+ (* DeltaSeconds -50.0) (`self.xPosition`))))
        (`SceneComponent.K2_SetRelativeLocation` (`self.Sphere`) (`KismetMathLibrary.MakeVector` _output_get_2) false false)
        (if (<= (`self.xPosition`) 0.0)
          (set `self.isLPosMovement` true))))))

(fn `Play`
  (params (isPlay :type Boolean))
  (returns (bResult :type Boolean))
  (set `self.isPlay` isPlay)
  (return false))

(fn `UserConstructionScript`)