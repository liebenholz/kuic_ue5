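; Actor Blueprint that moves its Sphere component in a repeating square loop in the relative XZ plane.
; Tick switches on a MoveType state (Right, Up, Left, Down), stepping XPosition or ZPosition at a constant delta-time-scaled speed and applying it as the Sphere's relative location.
; Each state advances to the next when its axis reaches the square's bound, with a zero-length Delay ahead of every step.
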(event `self.ReceiveBeginPlay`)

(event `self.ReceiveTick`
  (params (DeltaSeconds :type "Float (single-precision)"))
  (switch `/Game/EN_moveType` (`self.moveType`)
    (:`NewEnumerator0`
      ;[1 1 1] 오른족으로 움직이기
      (`KismetSystemLibrary.Delay` 0.0)
      (bind _output_get (set `self.xPosition` (+ (* DeltaSeconds 50.0) (`self.xPosition`))))
      (`SceneComponent.K2_SetRelativeLocation` (`self.Sphere`) (`KismetMathLibrary.MakeVector` _output_get 0.0 (`self.zPosition`)) false false)
      (if (>= (`self.xPosition`) 100.0)
        (set `self.moveType` "NewEnumerator1")))
    (:`NewEnumerator1`
      ;[1 1 1] 위쪽으로 움직이기
      (`KismetSystemLibrary.Delay` 0.0)
      (bind _output_get_2 (set `self.zPosition` (+ (* DeltaSeconds 50.0) (`self.zPosition`))))
      (`SceneComponent.K2_SetRelativeLocation` (`self.Sphere`) (`KismetMathLibrary.MakeVector` (`self.xPosition`) 0.0 _output_get_2) false false)
      (if (>= (`self.zPosition`) 100.0)
        (set `self.moveType` "NewEnumerator2")))
    (:`NewEnumerator2`
      ;[1 1 1] 왼쪽으로 한 번 움직이기
      (`KismetSystemLibrary.Delay` 0.0)
      (bind _output_get_3 (set `self.xPosition` (+ (* DeltaSeconds -50.0) (`self.xPosition`))))
      (`SceneComponent.K2_SetRelativeLocation` (`self.Sphere`) (`KismetMathLibrary.MakeVector` _output_get_3 0.0 (`self.zPosition`)) false false)
      (if (<= (`self.xPosition`) 0.0)
        (set `self.moveType` "NewEnumerator3")))
    (:`NewEnumerator3`
      ;[1 1 1] 아래쪽으로 한 번 움직이기
      (`KismetSystemLibrary.Delay` 0.0)
      (bind _output_get_4 (set `self.zPosition` (+ (* DeltaSeconds -50.0) (`self.zPosition`))))
      (`SceneComponent.K2_SetRelativeLocation` (`self.Sphere`) (`KismetMathLibrary.MakeVector` (`self.xPosition`) 0.0 _output_get_4) false false)
      (if (<= (`self.zPosition`) 0.0)
        (set `self.moveType` "NewEnumerator0")))))

(fn `UserConstructionScript`)